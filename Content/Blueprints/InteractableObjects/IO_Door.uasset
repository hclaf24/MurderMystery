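; IO_Door is an interactable door Blueprint that swings open and closed.
; InteractionEvent and DialogueEvent share one toggle that flips the Open flag and plays or reverses the OpenDoor timeline.
; The timeline's Yaw track is multiplied by OpenAngle to set the mesh's relative yaw, so closing retraces the opening swing.
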(event `self.Interaction Event`
  (bind _returnvalue (not (`self.Open?`)))
  (if _returnvalue :!label _label
    (set `self.Open?` _returnvalue)
    (bind (_direction _yaw) (`Timeline|Open Door` :!label _label_2)
      (:`Update`
        (`SceneComponent.K2_SetRelativeRotation` (`self.Mesh`) (`KismetMathLibrary.MakeRotator` 0.0 0.0 (* _yaw (`self.Open Angle`))) false false)))
    (else
      (set `self.Open?` _returnvalue)
      (goto _label_2 :!via `Reverse`))))

(event `self.Dialogue Event`
  (goto _label))

(fn `UserConstructionScript`
  (`parent.UserConstructionScript`))