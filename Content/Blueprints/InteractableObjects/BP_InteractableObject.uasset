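; Base interactable object for a narrative template, with interaction and dialogue events that child Blueprints override.
; Capsule overlap with the player plus mouse-over state toggles the prompt widget and custom-depth rendering.
; AcceptInput fires InteractionEvent only when interactable, in range and moused over.
; Named objects bind to the dialogue controller's event dispatcher, falling back to a found controller with a warning if unset.
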(event `self.ReceiveBeginPlay`
  ;[1 0 0.375] get player character at start of game
  (`self.Set interact text`)
  (bind _aschar_narrative_template (cast `/Game/Blueprints/Char_NarrativeTemplate` (`GameplayStatics.GetPlayerCharacter` 0)))
  (set `self.PlayerCharacter` _aschar_narrative_template)
  (set `self.Player Camera` (`/Game/Blueprints/Char_NarrativeTemplate.FirstPersonCamera` _aschar_narrative_template))
  (bind _aspc_narrative_template (cast `/Game/Blueprints/PC_NarrativeTemplate` (`GameplayStatics.GetPlayerController` 0)))
  (set `self.Player Controller` _aspc_narrative_template)
  (`|ExecutionSequence`
    (:`then_0`
      ;[0 0.2734 1] Check the dialogue controller's ref
      (`/Engine/EditorBlueprintResources/StandardMacros.IsValid` (`self.DialogueController Ref`)
        (:`Is Not Valid`
          (bind _outactors (`GameplayStatics.GetAllActorsOfClass` "/Game/Blueprints/DialogueSystem/BP_DialogueController.BP_DialogueController_C")) ; The dialogue controller ref should be set manually, but if it's not then automatically pick one and set the ref
          (for _array_element _outactors
            (set `self.DialogueController Ref` _array_element))
          (`KismetSystemLibrary.PrintString` (`KismetTextLibrary.Conv_TextToString` (`|FormatText` "WARNING: Dialogue controller ref not set in interactable object [{object_name}]. Please set the reference in {object_name}'s details panel." (`KismetTextLibrary.Conv_StringToText` (`KismetSystemLibrary.GetDisplayName` self)))) true true (struct :`G` 0.66 :`B` 1.0 :`A` 1.0) 10.0))))
    (:`then_1`
      ;[1 0 0.6094] Register this object's dialogue event to the dialogue controller's event dispatcher
      (if (not (`KismetStringLibrary.EqualEqual_StrStr` (`self.DialogueEventName`)))
        (add `/Game/Blueprints/DialogueSystem/BP_DialogueController.DialogueEvent` (`self.DialogueController Ref`) (delegate `Check Dialogue Event Received`))))))

(event `self.Capsule.OnComponentBeginOverlap`
  (params (OverlappedComponent :type "PrimitiveComponent Object Reference") (OtherActor :type "Actor Object Reference") (OtherComp :type "PrimitiveComponent Object Reference") (OtherBodyIndex :type Integer) (bFromSweep :type Boolean) (SweepResult :type "HitResult Structure (by ref)"))
  ;[0 1 0.8594] Begin/End overlap
  (if (== OtherActor (`self.PlayerCharacter`))
    (set `self.In Range?` true)
    (if (`self.Mouse Over?`)
      (`self.Change Interactable` true))))

(event `Check Dialogue Event Received`
  (params (`Event Name` :type String))
  ;[1 0 0.6094] Register this object's dialogue event to the dialogue controller's event dispatcher
  (if (`KismetStringLibrary.EqualEqual_StrStr` `Event Name` (`self.DialogueEventName`))
    (`self.Dialogue Event`)))

(event `self.Capsule.OnComponentEndOverlap`
  (params (OverlappedComponent :type "PrimitiveComponent Object Reference") (OtherActor :type "Actor Object Reference") (OtherComp :type "PrimitiveComponent Object Reference") (OtherBodyIndex :type Integer))
  ;[0 1 0.8594] Begin/End overlap
  (if (== OtherActor (`self.PlayerCharacter`))
    (set `self.In Range?` false)
    (`self.Change Interactable` false)))

(event `Interaction Event`
  ;[1 0 0.4687] Events to override in child blueprints
  (`KismetSystemLibrary.PrintString` "WARNING: Calling an interaction event on an object that has not specified an Interaction Event override!" true true (struct :`G` 0.66 :`B` 1.0 :`A` 1.0) 10.0))

(event `Dialogue Event`
  ;[1 0 0.4687] Events to override in child blueprints
  (`KismetSystemLibrary.PrintString` "WARNING: Calling a dialogue event on an object that has not specified an dialogue Event override!" true true (struct :`G` 0.66 :`B` 1.0 :`A` 1.0) 10.0))

(fn `Accept Input`
  (if (`self.Am Interactable?`)
    (if (`self.In Range?`)
      (if (`self.Mouse Over?`)
        (`self.Interaction Event`)))))

(fn `Become Inactive`
  (set `self.Am Active?` false)
  (set `self.Am Interactable?` false)
  (`SceneComponent.SetHiddenInGame` (`self.Interact Text`) true false))

(fn `Begin Mouse Over`
  (set `self.Mouse Over?` true)
  (if (`self.In Range?`)
    (`self.Change Interactable` true)))

(fn `Change Interactable`
  (params (`Interactable?` :type Boolean))
  (bind _mesh (`self.Mesh`))
  (if (`self.Am Active?`)
    (if `Interactable?`
      (`SceneComponent.SetHiddenInGame` (`self.Interact Text`) false false)
      (set `self.Am Interactable?` true)
      (`PrimitiveComponent.SetRenderCustomDepth` _mesh true)
      (else
        (`SceneComponent.SetHiddenInGame` (`self.Interact Text`) true false)
        (set `self.Am Interactable?` false)
        (`PrimitiveComponent.SetRenderCustomDepth` _mesh false)))))

(fn `End Mouse Over`
  (set `self.Mouse Over?` false)
  (`self.Change Interactable` false))

(fn `Set interact text`
  (bind _aswb_interactable_object_text (cast `/Game/Blueprints/InteractableObjects/WB_InteractableObjectText` (`WidgetComponent.GetUserWidgetObject` (`self.Interact Text`))))
  (`TextBlock.SetText` (`/Game/Blueprints/InteractableObjects/WB_InteractableObjectText.InteractionText` _aswb_interactable_object_text) (`self.InteractionText`)))

(fn `UserConstructionScript`
  (`CapsuleComponent.SetCapsuleRadius` (`self.Capsule`) (`self.InteractionRadius`) true)
  (`BoxComponent.SetBoxExtent` (`self.MouseOverBox`) (`self.Mouse Over Dimensions`) true))