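; Dialogue controller that queues dialogue data tables and plays each row by row, following goto row names for branching.
; Lines route to debug log, phone, thoughts, TV or computer with post-delays, while Event rows trigger named world events.
; Input rows gather following prompts for the player controller's UI, then a Tick timer auto-selects the last prompt if no choice arrives.
; EOF rows release the controller to start the next queued table.
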(event `self.ReceiveBeginPlay`
  ;[1 0.9844 0] Get character and controller on beginplay
  (bind _aschar_narrative_template (cast `/Game/Blueprints/Char_NarrativeTemplate` (`GameplayStatics.GetPlayerCharacter` 0)))
  (set `self.PlayerCharacter` _aschar_narrative_template)
  (bind _aspc_narrative_template (cast `/Game/Blueprints/PC_NarrativeTemplate` (`GameplayStatics.GetPlayerController` 0)))
  (set `self.PlayerController` _aspc_narrative_template))

(event `Add Dialogue to Queue`
  (params (`Dialogue table` :type "DataTable Object Reference"))
  ;[1 0 0.7734] Accept new dialogue and add to queue
  (`KismetArrayLibrary.Array_Add` (`self.DialogueQueue`) `Dialogue table`)
  (if (not (`self.IsAlreadyActive?`))
    (`self.Step through Dialogue Queue`)))

(event `Step through Dialogue Queue`
  (bind _dialoguequeue (`self.DialogueQueue`))
  ;[0.9922 1 0] Pop the bottom item in the dialogue queue
  (if (`KismetArrayLibrary.Array_IsValidIndex` _dialoguequeue)
    (set `self.CurrentDialogueTable` (`|GetArrayItem` _dialoguequeue))
    (`KismetArrayLibrary.Array_Remove` _dialoguequeue)
    (`self.Read Dialogue Table`)))

(event `Read Dialogue Table`
  ;[1 0.4688 0] Initialize data reading loop
  (if (`self.IsAlreadyActive?`)
    (`KismetSystemLibrary.PrintString` "WARNING: Tried to read a new dialogue table, but there is one already active!")
    (else
      (set `self.IsAlreadyActive?` true)
      (set `self.CurrentLineIndex` 0)
      (bind _outrownames (`DataTableFunctionLibrary.GetDataTableRowNames` (`self.CurrentDialogueTable`)))
      (set `self.RowNames` _outrownames) ; Use this array of names to get each row line-by-line
      (`self.Read Next Dialogue Line`))))

(event `Read Next Dialogue Line`
  (bind (_currlinedata_messagetype _currlinedata_destination _currlinedata_speaker _currlinedata_postdelay _currlinedata_message) (break `/Game/Blueprints/DialogueSystem/Struct_LineData` (`self.CurrLineData`)))
  (bind _currentlineindex (`self.CurrentLineIndex`))
  (bind (_currlinedata_messagetype_2 _currlinedata_destination_2 _currlinedata_speaker_2 _currlinedata_postdelay_2 _currlinedata_message_2 _currlinedata_gotorowname) (break `/Game/Blueprints/DialogueSystem/Struct_LineData` (`self.CurrLineData`)))
  (bind _currlinedata_messagetype_3 (break `/Game/Blueprints/DialogueSystem/Struct_LineData` (`self.CurrLineData`)))
  (bind (_currlinedata_messagetype_4 _currlinedata_destination_3 _currlinedata_speaker_3 _currlinedata_postdelay_3 _currlinedata_message_3) (break `/Game/Blueprints/DialogueSystem/Struct_LineData` (`self.CurrLineData`)))
  (bind _output (`|GetArrayItem` (`self.RowNames`) _currentlineindex))
  ;[0.03125 0 1] Read through dialogue lines
  ;;[1 0 0.5625] Get the current line's data
  (bind _returnvalue (`|GetDataTableRow` (`self.CurrentDialogueTable`) _output)
    (:`then`
      (set `self.CurrLineData` _returnvalue)
      ;;[0.1016 0 1] Check Goto value
      (if (== _currlinedata_gotorowname "None")
        (`/Engine/EditorBlueprintResources/StandardMacros.IncrementInt` (`self.CurrentLineIndex`)
          (:`  `
            _))
        (else
          (set `self.CurrentLineIndex` (`KismetArrayLibrary.Array_Find` (`self.RowNames`) _currlinedata_gotorowname))))
      ;;[0.4766 1 0] Check line type
      (switch `/Game/Blueprints/DialogueSystem/Enum_LineTypes` _currlinedata_messagetype_3
        (:`NewEnumerator0`
          ;;[0.7109 0 1] Handle Outputting lines
          (`self.Send Line to Destination` _currlinedata_message_3 _currlinedata_destination_3 _currlinedata_speaker_3)
          (`KismetSystemLibrary.Delay` _currlinedata_postdelay_3)
          (`self.Read Next Dialogue Line`))
        (:`NewEnumerator1`
          ;;[0.1719 1 0] Handle Prompt type input error
          (`KismetSystemLibrary.PrintString` (`KismetTextLibrary.Conv_TextToString` (`|FormatText` "ERROR: Prompt sent to output on row #{row} " (`KismetTextLibrary.Conv_StringToText` (`KismetStringLibrary.Conv_IntToString` (`self.CurrentLineIndex`))))) true true (struct :`G` 0.66 :`B` 1.0 :`A` 1.0) 20.0))
        (:`NewEnumerator2`
          ;;[0.125 1 0] Read the next few prompt lines until End input detected then break out of loop
          (`self.Read Prompts` (`self.CurrentLineIndex`)) ; Note: Curr line already incremented, starting line is 1st prompt
          (`self.Send Input Prompts`)
          (bind _aspc_narrative_template (cast `/Game/Blueprints/PC_NarrativeTemplate` (`GameplayStatics.GetPlayerController` 0)))
          (`/Game/Blueprints/PC_NarrativeTemplate.Set Dialogue Input Location` _aspc_narrative_template self)
          (`self.Start Waiting for Input`))
        (:`NewEnumerator3`
          ;;[0.1719 1 0] Handle End Input type error
          (`KismetSystemLibrary.PrintString` (`KismetTextLibrary.Conv_TextToString` (`|FormatText` "ERROR: End of input sent to output on row {row} " (`KismetTextLibrary.Conv_StringToText` (`KismetStringLibrary.Conv_IntToString` (`self.CurrentLineIndex`))))) true true (struct :`G` 0.66 :`B` 1.0 :`A` 1.0) 20.0))
        (:`NewEnumerator5`
          ;;[0.4531 1 0] Call world events from dialogue
          (`self.DialogueEvent` (`KismetTextLibrary.Conv_TextToString` _currlinedata_message)) ; This calls the "Dialogue Event" event on any interactable objects whose "Dialogue Event" variable matches the "Event Name" string
          (`self.Read Next Dialogue Line`))
        (:`NewEnumerator4`
          ;;;[0 1 0.1562] EOF Reached
          (set `self.IsAlreadyActive?` false)
          (`self.Step through Dialogue Queue`) ; Check if there is any dialogue waiting in the queue
        )))
    (:`RowNotFound`
      (`KismetSystemLibrary.PrintString` (`KismetTextLibrary.Conv_TextToString` (`|FormatText` "ERROR: row #{row}, name {name} was not found!" (`KismetTextLibrary.Conv_NameToText` _output) (`KismetTextLibrary.Conv_IntToText` _currentlineindex))) true true (struct :`G` 0.66 :`B` 1.0 :`A` 1.0) 20.0))))

(event `Start Waiting for Input`
  ;[1 0.8438 0] Handle Player input for prompts
  ;;[1 0 0.4922] Start waiting for prompt input
  (set `self.InputTimeCounter` 0.0)
  (set `self.WaitingForInput?` true))

(event `Receive Input`
  (params (`Input Number` :type Integer))
  ;[1 0.8438 0] Handle Player input for prompts
  ;;[1 0 0.1406] Get input from the player and choose a prompt
  (if (and (`self.WaitingForInput?`) (>= `Input Number` 1) (<= (- `Input Number` 1) (`KismetArrayLibrary.Array_Length` (`self.PromptGotos`))))
    (`self.Choose Prompt` (- `Input Number` 1))))

(event `self.ReceiveTick`
  (params (DeltaSeconds :type "Float (single-precision)"))
  (bind _returnvalue (`KismetArrayLibrary.Array_LastIndex` (`self.PromptGotos`)))
  ;[1 0.8438 0] Handle Player input for prompts
  ;;[0 1 0.7188] Count down input timer, call last prompt otherwise
  (if (`self.WaitingForInput?`)
    (if (> (`self.InputTimeCounter`) (`self.InputTimeOut`))
      (`/Game/UI/WB_GameplayUI.Choose Prompt UI` (`/Game/Blueprints/PC_NarrativeTemplate.Gameplay UI` (`self.PlayerController`)) (+ _returnvalue 1)) ; Need to manually tell the UI to choose the final prompt
      (`self.Choose Prompt` _returnvalue)
      (else
        (set `self.InputTimeCounter` (+ DeltaSeconds (`self.InputTimeCounter`)))))))

(event `Choose Prompt`
  (params (`Prompt Index` :type Integer))
  ;[1 0.8438 0] Handle Player input for prompts
  ;;[0.9453 1 0] Choose one of the provided prompts, wait for its delay, then go to the specified line
  (bind _returnvalue (`|GetDataTableRow` (`self.CurrentDialogueTable`) (`|GetArrayItem` (`self.RowNames`) (+ (`self.CurrentLineIndex`) `Prompt Index`))) ; Get the data table entry for the chosen prompt
    (:`then`
      (set `self.CurrentLineIndex` (`KismetArrayLibrary.Array_Find` (`self.RowNames`) (`|GetArrayItem` (`self.PromptGotos`) `Prompt Index`)))
      (set `self.WaitingForInput?` false)
      (`KismetSystemLibrary.Delay` (`.PostDelay_7_4CA4D09E4FFBD945E985AF8DBBB8F823` (break `/Game/Blueprints/DialogueSystem/Struct_LineData` _returnvalue))) ; Read the delay from the chosen prompt
      (`self.Read Next Dialogue Line`))
    (:`RowNotFound`
      (`KismetSystemLibrary.PrintString` "ERROR: Invalid row found when reading prompt delays!"))))

(fn `Read Prompts`
  (params (`Starting Line` :type Integer))
  (locals (Local_CurrLine :type Integer) (`EndInput Reached?` :type Boolean))
  (set `local.Local_CurrLine` `Starting Line`)
  (`KismetArrayLibrary.Array_Clear` (`self.PromptsArray`))
  (`KismetArrayLibrary.Array_Clear` (`self.PromptGotos`))
  (while (not (`local.EndInput Reached?`))
    (`|ExecutionSequence`
      (:`then_0`
        (bind _returnvalue (`|GetDataTableRow` (`self.CurrentDialogueTable`) (`|GetArrayItem` (`self.RowNames`) (`local.Local_CurrLine`)))
          (:`then`
            (bind (_messagetype _destination _speaker _postdelay _message _gotorowname) (break `/Game/Blueprints/DialogueSystem/Struct_LineData` _returnvalue))
            (switch `/Game/Blueprints/DialogueSystem/Enum_LineTypes` _messagetype
              (:`NewEnumerator0`
                ;[0.1719 1 0] Handle Input order error
                (`KismetSystemLibrary.PrintString` (`KismetTextLibrary.Conv_TextToString` (`|FormatText` "ERROR: Encountered non-prompt or extra input while reading prompts on row {row} " (`KismetTextLibrary.Conv_StringToText` (`KismetStringLibrary.Conv_IntToString` (`self.CurrentLineIndex`))))) true true (struct :`G` 0.66 :`B` 1.0 :`A` 1.0) 20.0 :!label _label))
              (:`NewEnumerator1`
                ;[0 1 0.1328] Add prompts to array until end input reached
                (`KismetArrayLibrary.Array_Add` (`self.PromptsArray`) _message)
                (`KismetArrayLibrary.Array_Add` (`self.PromptGotos`) _gotorowname))
              (:`NewEnumerator2`
                (goto _label))
              (:`NewEnumerator3`
                (set `local.EndInput Reached?` true))
              (:`NewEnumerator4`
                (goto _label))))))
      (:`then_1`
        (`/Engine/EditorBlueprintResources/StandardMacros.IncrementInt` (`local.Local_CurrLine`))))))

(fn `Send Input Prompts`
  (`/Game/Blueprints/PC_NarrativeTemplate.Send prompts to Gameplay UI` (`self.PlayerController`) (`self.PromptsArray`) (`self.InputTimeOut`)))

(fn `Send Line to Destination`
  (params (`Line text` :type Text) (Destination :type "/Game/Blueprints/DialogueSystem/Enum_Destinations Enum" :default "NewEnumerator0") (Speaker :type "/Game/Blueprints/DialogueSystem/Enum_Speakers Enum" :default "NewEnumerator0"))
  (locals (L_Text :type Text) (L_Speaker :type "/Game/Blueprints/DialogueSystem/Enum_Speakers Enum"))
  (bind _returnvalue (`KismetTextLibrary.Conv_TextToString` (`local.L_Text`)))
  (set `local.L_Text` `Line text`)
  (set `local.L_Speaker` Speaker)
  (switch `/Game/Blueprints/DialogueSystem/Enum_Destinations` Destination
    (:`NewEnumerator0`
      ;[1 0.2109 0] Debug
      (switch `/Game/Blueprints/DialogueSystem/Enum_Speakers` (`local.L_Speaker`)
        (:`NewEnumerator0`
          (`KismetSystemLibrary.PrintString` _returnvalue true true (struct :`G` 0.66 :`B` 1.0 :`A` 1.0) 10.0))
        (:`NewEnumerator1`
          (`KismetSystemLibrary.PrintString` _returnvalue true true (struct :`R` 1.0 :`G` 0.060419 :`B` 0.120146 :`A` 1.0) 10.0))))
    (:`NewEnumerator1`
      ;[1 0.5156 0] Phone
      (`/Game/Blueprints/PC_NarrativeTemplate.Send lines to phone` (`self.PlayerController`) (`local.L_Text`) (`local.L_Speaker`)))
    (:`NewEnumerator2`
      ;[1 0.5391 0] Thoughts
      (`/Game/Blueprints/PC_NarrativeTemplate.Send lines to Thoughts` (`self.PlayerController`) (`local.L_Text`)))
    (:`NewEnumerator3`
      ;[0.9453 0 1] TV
      (`/Engine/EditorBlueprintResources/StandardMacros.IsValid` (`self.TV`)
        (:`Is Valid`
          (`/Game/Blueprints/InteractableObjects/IO_TV.Add TV text` (`self.TV`) (`local.L_Text`) :!label _label))
        (:`Is Not Valid`
          (bind _outactors (`GameplayStatics.GetAllActorsOfClass` "/Game/Blueprints/InteractableObjects/IO_TV.IO_TV_C"))
          (for _array_element _outactors
            (bind _asio_tv (cast `/Game/Blueprints/InteractableObjects/IO_TV` _array_element))
            (set `self.TV` _asio_tv)
            (goto _label)))))
    (:`NewEnumerator4`
      ;[0.9688 1 0] Computer
      (`/Engine/EditorBlueprintResources/StandardMacros.IsValid` (`self.Computer`)
        (:`Is Valid`
          _)
        (:`Is Not Valid`
          (bind _outactors_2 (`GameplayStatics.GetAllActorsOfClass` "/Game/Blueprints/InteractableObjects/IO_Computer.IO_Computer_C"))
          (for _array_element_2 _outactors_2
            (bind _asio_computer (cast `/Game/Blueprints/InteractableObjects/IO_Computer` _array_element_2))
            (set `self.Computer` _asio_computer))))
      (`/Game/Blueprints/InteractableObjects/IO_Computer.Add Computer text` (`self.Computer`) (`local.L_Text`)))))

(fn `UserConstructionScript`)