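; Player controller for a narrative template that links dialogue logic to the gameplay HUD.
; It creates the gameplay UI widget on BeginPlay, or on demand, and forwards phone texts, thoughts and timed prompts to it.
; Three dialogue input actions send the chosen prompt number to a registered dialogue controller and update the UI to show the choice.
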(event `self.ReceiveBeginPlay`
  ;[0.6641 1 0] BeginPlay
  (`self.Create Gameplay UI`))

(event `InputAction|DL_Input1`
  (params (Key :type "Key Structure"))
  (bind _dialogue_input_bp (`self.Dialogue Input BP`))
  (bind _chosen_prompt (`self.Chosen Prompt`))
  ;[0 1 0.6016] Send dialogue inputs (2 options)
  (:`Pressed`
    (set `self.Chosen Prompt` 1)
    (`/Engine/EditorBlueprintResources/StandardMacros.IsValid` _dialogue_input_bp :!label _label
      (:`Is Valid`
        (`/Game/Blueprints/DialogueSystem/BP_DialogueController.Receive Input` _dialogue_input_bp _chosen_prompt)
        (`/Game/UI/WB_GameplayUI.Choose Prompt UI` (`self.Gameplay UI`) _chosen_prompt)))))

(event `InputAction|DL_Input2`
  (params (Key :type "Key Structure"))
  ;[0 1 0.6016] Send dialogue inputs (2 options)
  (:`Pressed`
    (set `self.Chosen Prompt` 2)
    (goto _label)))

(event `InputAction|DL_Input3`
  (params (Key :type "Key Structure"))
  ;[0 1 0.6016] Send dialogue inputs (2 options)
  (:`Pressed`
    (set `self.Chosen Prompt` 3)
    (goto _label)))

(event `Send lines to phone`
  (params (`Line Text` :type Text) (Speaker :type "/Game/Blueprints/DialogueSystem/Enum_Speakers Enum" :default "NewEnumerator0"))
  (bind _gameplay_ui (`self.Gameplay UI`))
  ;[0.8047 1 0] Send phone texts to gameplay UI
  (`/Engine/EditorBlueprintResources/StandardMacros.IsValid` _gameplay_ui
    (:`Is Valid`
      _)
    (:`Is Not Valid`
      (`self.Create Gameplay UI`)))
  (`/Game/UI/WB_GameplayUI.Add Phone Text` _gameplay_ui `Line Text` Speaker))

(event `Send lines to Thoughts`
  (params (`New Text` :type Text))
  (bind _gameplay_ui (`self.Gameplay UI`))
  ;[1 0 0.4453] Send thoughts to gameplay UI
  (`/Engine/EditorBlueprintResources/StandardMacros.IsValid` _gameplay_ui
    (:`Is Valid`
      _)
    (:`Is Not Valid`
      (`self.Create Gameplay UI`)))
  (`/Game/UI/WB_GameplayUI.Add Thought Text` _gameplay_ui `New Text`))

(event `Send prompts to Gameplay UI`
  (params (`Prompt lines` :type "Array of Text") (`Input time out` :type "Float (double-precision)"))
  (bind _gameplay_ui (`self.Gameplay UI`))
  ;[1 0 0] Send prompts to screen
  (`/Engine/EditorBlueprintResources/StandardMacros.IsValid` _gameplay_ui
    (:`Is Valid`
      _)
    (:`Is Not Valid`
      (`self.Create Gameplay UI`)))
  (`/Game/UI/WB_GameplayUI.Send prompts` _gameplay_ui `Prompt lines` `Input time out`))

(fn `Create Gameplay UI`
  (`/Engine/EditorBlueprintResources/StandardMacros.IsValid` (`self.Gameplay UI`)
    (:`Is Not Valid`
      (bind _returnvalue (`|CreateWidget` "/Game/UI/WB_GameplayUI.WB_GameplayUI_C"))
      (bind _output_get (set `self.Gameplay UI` _returnvalue))
      (`UserWidget.AddToViewport` _output_get 0))))

(fn `Set Dialogue Input Location`
  (params (`Dialogue Controller` :type "/Game/Blueprints/DialogueSystem/BP_DialogueController Object Reference"))
  (set `self.Dialogue Input BP` `Dialogue Controller`))

(fn `UserConstructionScript`)